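; Behavior tree task that makes an AI-controlled ThirdPerson_BP pawn aim and shoot at its target.
; On execute it sets the pawn's Aiming and Shooting flags and focuses the controller on the blackboard Target actor.
; It never calls FinishExecute, so it keeps running until aborted, when it clears both flags and the focus, then finishes the abort.
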(event `self.ReceiveExecuteAI`
  (params (OwnerController :type "AIController Object Reference") (ControlledPawn :type "Pawn Object Reference"))
  ;[1 1 1] Update
  (`|ExecutionSequence`
    (:`then_0`
      (bind _asthird_person_bp (cast `/Game/Static/Blueprints/ThirdPerson_BP` ControlledPawn))
      (set `/Game/Static/Blueprints/ThirdPerson_BP.Aiming` true _asthird_person_bp)
      (set `/Game/Static/Blueprints/ThirdPerson_BP.Shooting` true _asthird_person_bp))
    (:`then_1`
      (`AIController.K2_SetFocus` OwnerController (`BTFunctionLibrary.GetBlackboardValueAsActor` (`self.Target`))))))

(event `self.ReceiveAbortAI`
  (params (OwnerController :type "AIController Object Reference") (ControlledPawn :type "Pawn Object Reference"))
  ;[1 1 1] Abort AI
  (`|ExecutionSequence`
    (:`then_0`
      (bind _asthird_person_bp (cast `/Game/Static/Blueprints/ThirdPerson_BP` ControlledPawn))
      (set `/Game/Static/Blueprints/ThirdPerson_BP.Aiming` false _asthird_person_bp)
      (set `/Game/Static/Blueprints/ThirdPerson_BP.Shooting` false _asthird_person_bp))
    (:`then_1`
      (`AIController.K2_ClearFocus` OwnerController)
      (`self.FinishAbort`))))