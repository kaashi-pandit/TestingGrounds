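; NPC AI controller that starts the Patrol behavior tree on the PatrolData blackboard at BeginPlay.
; AI perception updates only print a debug string naming the pawn, the perceived actor and the stimulus's sense class.
; FindPatrolRoute writes the first PatrolPoints entry of the controlled ThirdPersonCharacter to the Waypoint key of a given blackboard, and is not called within this graph.
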(event `self.ReceiveBeginPlay`
  (`self.UseBlackboard` "/Game/Blueprints/PatrolData.PatrolData")
  (`self.RunBehaviorTree` "/Game/Blueprints/Patrol.Patrol"))

(event `self.AIPerception.OnTargetPerceptionUpdated`
  (params (Actor :type "Actor Object Reference") (Stimulus :type "AIStimulus Structure"))
  (bind _returnvalue (`AIPerceptionSystem.GetSenseClassForStimulus` Stimulus))
  (`KismetSystemLibrary.PrintString` (`KismetStringLibrary.Concat_StrStr` (`KismetSystemLibrary.GetDisplayName` (`self.K2_GetPawn`)) " is seeing " (`KismetSystemLibrary.GetDisplayName` Actor) " by stimulus " (`KismetSystemLibrary.GetClassDisplayName` _returnvalue))))

(fn `FindPatrolRoute`
  (params (Blackboard :type "BlackboardComponent Object Reference"))
  (bind _asthird_person_character (cast `/Game/ThirdPersonBP/Blueprints/ThirdPersonCharacter` (`self.K2_GetPawn`)))
  (`BlackboardComponent.SetValueAsObject` Blackboard "Waypoint" (`|GetArrayItem` (`/Game/ThirdPersonBP/Blueprints/ThirdPersonCharacter.PatrolPoints` _asthird_person_character))))

(fn `UserConstructionScript`)